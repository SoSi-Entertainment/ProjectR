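; Interaction area actor that marks a zone tied to a worker, taken from its attach parent actor on BeginPlay.
; Its root uses absolute location, so its position does not follow the parent, and Tick draws a debug line from worker to area.
; A box overlap test on the player pawn sets the text render's visibility through a SetVisibility event and is the result Interact returns.
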(event Custom|Set%20Visibility
  ;[1 1 1] Show area text
  (bind _result (CallFunction|IsPlayerinCollisionBox))
  (Rendering|SetVisibility (Variables|Default|GetText%20render) _result false))

(event EventBeginPlay
  ;[1 1 1] Set attached worker
  (Variables|Default|Setworker (Actor|GetAttachParentActor)))

(event Collision|EventActorBeginOverlap
  (params (OtherActor :type Actor%20Object%20Reference)))

(event EventTick
  (params (DeltaSeconds :type Float%20%28single-precision%29))
  (bind _worker (Variables|Default|Getworker))
  ;[1 1 1] Draw line to warker
  (Utilities|IsValid _worker
    (:Is%20Valid
      (Rendering|Debug|DrawDebugLine (Transformation|GetActorLocation _worker) (Transformation|GetActorLocation) "(R=0.000000,G=0.455463,B=1.000000,A=1.000000)" 0.0 2.0))))

(fn ConstructionScript
  (Transformation|SetAbsolute (Variables|Default|GetDefaultSceneRoot) true false false))

(fn IsPlayerinCollisionBox
  (return (Collision|IsOverlappingActor (Variables|Default|GetBox%20collision) (Game|Player|GetPlayerPawn 0) :!class /Script/Engine.PrimitiveComponent)))

(fn Interact
  (bind _result (CallFunction|IsPlayerinCollisionBox))
  (return _result))