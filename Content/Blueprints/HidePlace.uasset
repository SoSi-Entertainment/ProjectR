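; HidePlace is an overlap-triggered area actor, named as a hiding spot, that shows a text label while a qualifying actor is inside.
; Begin and end overlap call the parent logic, then set IsActive for actors deriving from DetectionClass and apply it to the TextRender visibility.
; The construction script calls Set on SetterZeroX.
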(event EventBeginPlay)

(event Collision|EventActorBeginOverlap
  (params (OtherActor :type Actor%20Object%20Reference))
  ;[1 1 1] Show area text
  (|CallParentFunction OtherActor)
  (if (Utilities|ClassIsChildOf (Utilities|GetClass OtherActor) (Variables|Default|GetDetectionClass))
    (Variables|Default|SetIsActive true)
    (Rendering|SetVisibility (Variables|Default|GetText%20render) (Variables|Default|GetIsActive) false)))

(event EventTick
  (params (DeltaSeconds :type Float%20%28single-precision%29)))

(event Collision|EventActorEndOverlap
  (params (OtherActor :type Actor%20Object%20Reference))
  ;[1 1 1] Show area text
  (|CallParentFunction OtherActor)
  (if (Utilities|ClassIsChildOf (Utilities|GetClass OtherActor) (Variables|Default|GetDetectionClass))
    (Variables|Default|SetIsActive false)
    (Rendering|SetVisibility (Variables|Default|GetText%20render) (Variables|Default|GetIsActive) false)))

(fn ConstructionScript
  (Default|Set (Variables|Default|GetSetterZeroX)))