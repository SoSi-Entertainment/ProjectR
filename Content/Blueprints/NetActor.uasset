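; NetActor is an actor that forms a parent/child network from the editor or runtime attachment hierarchy, with an Interact function that returns false.
; On BeginPlay it caches its attached parent and direct children that are NetActors, printing warnings for other attached types.
; Tick draws a debug line to its net parent.
; The construction script can make the root's location absolute, so attachment need not affect placement.
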(event EventBeginPlay
  (bind _returnvalue (Actor|GetAttachParentActor))
  ;[1 1 1] Set net parent
  (Utilities|IsValid _returnvalue
    (:Is%20Valid
      (bind _asnet_actor (Utilities|Casting|CastToNetActor _returnvalue)
        (:then
          (Variables|Default|SetNetParent _asnet_actor))
        (:CastFailed
          (Development|PrintString (Utilities|String|Append "warning: \"" (Utilities|GetDisplayName self) "\" attached to not NetActor") true true "(R=0.796875,G=0.562865,B=0.000000,A=1.000000)" 1e+01))))
    (:Is%20Not%20Valid
      _))
  ;[1 1 1] Set net children
  (for _array_element (Actor|GetAttachedActors false false)
    (bind _asnet_actor_2 (Utilities|Casting|CastToNetActor _array_element)
      (:then
        (Utilities|Array|Add (Variables|Default|GetNetChildren) _asnet_actor_2))
      (:CastFailed
        (Development|PrintString (Utilities|String|Append "warning: to \"" (Utilities|GetDisplayName self) "\" attached not NetActor \"" (Utilities|GetDisplayName _array_element) "\"") true true "(R=0.796875,G=0.562865,B=0.000000,A=1.000000)" 1e+01)))))

(event Collision|EventActorBeginOverlap
  (params (OtherActor :type Actor%20Object%20Reference)))

(event EventTick
  (params (DeltaSeconds :type Float%20%28single-precision%29))
  (bind _netparent (Variables|Default|GetNetParent))
  ;[1 1 1] Draw line to net parent
  (Utilities|IsValid _netparent
    (:Is%20Valid
      (Rendering|Debug|DrawDebugLine (Transformation|GetActorLocation _netparent) (Transformation|GetActorLocation) "(R=0.000000,G=0.455463,B=1.000000,A=1.000000)" 0.0 2.0))))

(fn ConstructionScript
  (if (Variables|Default|GetPlacedAbsolute)
    (Transformation|SetAbsolute (Variables|Default|GetDefaultSceneRoot) true false false)))

(fn Interact
  (return false))