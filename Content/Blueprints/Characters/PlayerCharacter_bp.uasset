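; Player character Blueprint that handles interaction, pickups, hiding, energy and respawning.
; The interact input clicks overlapping IClickable actors, while beginning an overlap with an ICollectable collects it.
; Crouch toggles through the parent only inside a HidePlace, and leaving one while small toggles it back.
; Inputs adjust EnergyComponent or restart by destroying the pawn, which notifies MainGameMode_bp of death, then requesting a respawn for the cached controller.
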(event EventBeginPlay
  ;[1 1 1] Set up respawn
  (Variables|Default|SetControllerRef (Pawn|GetController)))

(event EventDestroyed
  ;[1 1 1] Set up respawn
  (bind _asmain_game_mode_bp (Utilities|Casting|CastToMainGameMode_bp (Game|GetGameMode)))
  (Default|CallOnPlayerDied _asmain_game_mode_bp self))

(event Collision|EventActorEndOverlap
  (params (OtherActor :type Actor%20Object%20Reference))
  (Utilities|Casting|CastToHidePlace OtherActor)
  (if (Variables|Default|GetisSmall)
    (|CallParentFunction)))

(event Collision|EventActorBeginOverlap
  (params (OtherActor :type Actor%20Object%20Reference))
  (bind _asicollectable (Utilities|Casting|CastToICollectable OtherActor))
  (Default|Collect _asicollectable self))

(event EventSwitchCrouch
  (bind _array_element (Utilities|Array|ForEachLoopwithBreak (Collision|GetOverlappingActors (Variables|Default|GetCapsuleComponent) "/Script/Engine.Actor" :!class /Script/Engine.PrimitiveComponent) :!label _label)
    (:LoopBody
      (Utilities|Casting|CastToHidePlace _array_element)
      (|CallParentFunction)
      (goto _label Break))))

(event Input|ActionEvents|InputActionRestart
  (params (Key :type Key%20Structure :default "None"))
  ;[1 1 1] Set up respawn
  (:Pressed
    (CallFunction|CallRestartPlayer)))

(event Input|ActionEvents|InputActionInteractAction
  (params (Key :type Key%20Structure :default "None"))
  ;[1 1 1] Click object
  (:Pressed
    (bind _array_element (Utilities|Array|ForEachLoopwithBreak (Collision|GetOverlappingActors (Variables|Default|GetCapsuleComponent) "/Script/Engine.Actor" :!class /Script/Engine.PrimitiveComponent) :!label _label)
      (:LoopBody
        (bind _asiclickable (Utilities|Casting|CastToIClickable _array_element))
        (Default|Click _asiclickable)
        (goto _label Break)))))

(event Input|ActionEvents|InputActionEnergy+
  (params (Key :type Key%20Structure :default "None"))
  (:Pressed
    (Default|PutEnergy (Variables|Default|GetEnergyComponent) 2e+01)))

(event Input|ActionEvents|InputActionEnergy-
  (params (Key :type Key%20Structure :default "None"))
  (:Pressed
    (Default|TakeEnerge (Variables|Default|GetEnergyComponent) 2e+01)))

(fn ConstructionScript)

(fn CallRestartPlayer
  (Actor|DestroyActor)
  (bind _asmain_game_mode_bp (Utilities|Casting|CastToMainGameMode_bp (Game|GetGameMode)))
  (Class|GameModeBase|RestartPlayer _asmain_game_mode_bp (Variables|Default|GetControllerRef)))

(fn Interact)