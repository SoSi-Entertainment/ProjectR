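; Enemy AI controller that chases the player within a trigger radius around its pawn while active.
; Each Tick compares distance to the player and issues AIMoveTo toward them, or otherwise toward the start location saved at BeginPlay.
; That return move has no Pawn input set.
; Debug drawing shows a cone at the start point and a radius circle, red for chase and green for return.
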(event EventBeginPlay
  (bind _output_get (Variables|Default|SetStartLocation (Transformation|GetActorLocation (Pawn|GetControlledPawn)))))

(event EventTick
  (params (DeltaSeconds :type Float%20%28single-precision%29))
  (bind _returnvalue (Game|Player|GetPlayerPawn 0))
  (bind _returnvalue_2 (Pawn|GetControlledPawn))
  (bind _triggerradius (Variables|Default|GetTriggerRadius))
  (bind _returnvalue_3 (Transformation|GetActorLocation _returnvalue_2))
  (Class|KismetSystemLibrary|DrawDebugConeinDegrees (+ (stale EventBeginPlay _output_get) "0,0,-44.000000") "0.000000, 0,-1.000000" 5e+01 3e+01 3e+01 50 "(R=1.000000,G=0.000000,B=0.000000,A=1.000000)" 0.0 1.0)
  (if (Utilities|IsValid _returnvalue)
    (Math|Float|CompareFloat (Math|Vector|Distance(Vector) (Transformation|GetActorLocation _returnvalue) _returnvalue_3) _triggerradius
      (:>
        (AI|AIMoveTo 0 (Variables|Default|GetStartLocation) 0 5.0 false :!label _label
          (:then
            (Rendering|Debug|DrawDebugCircle _returnvalue_3 _triggerradius 300 "(R=0.132879,G=1.000000,B=0.000000,A=1.000000)" 0.0 5.0 "0.000000,1.000000,0.000000" "0.000000,0.000000,1.000000"))))
      (:==
        (goto _label))
      (:<
        (if (Variables|Default|GetisActive)
          (AI|AIMoveTo _returnvalue_2 "0, 0, 0" _returnvalue 5.0 false
            (:then
              (Rendering|Debug|DrawDebugCircle _returnvalue_3 _triggerradius 300 "(R=1.000000,G=0.000000,B=0.008680,A=1.000000)" 0.0 5.0 "0.000000,1.000000,0.000000" "0.000000,0.000000,1.000000")))
          (else
            (goto _label)))))
    (else
      (goto _label))))

(fn ConstructionScript)