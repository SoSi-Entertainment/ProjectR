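; Lamp is a worker Blueprint that switches the material on its Cube between two looks as its inherited work functions run.
; Work0 applies MenuBallMaterial and Work1 applies CubeMaterial, each after calling the parent implementation.
; Interact defers to the parent and, when that returns true, clears Busy before passing the result back.
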(event EventBeginPlay
  (|CallParentFunction))

(event Collision|EventActorBeginOverlap
  (params (OtherActor :type Actor%20Object%20Reference))
  (|CallParentFunction OtherActor) ; This node is disabled and will not be called.\nDrag off pins to build functionality.
)

(event EventTick
  (params (DeltaSeconds :type Float%20%28single-precision%29))
  (|CallParentFunction DeltaSeconds) ; This node is disabled and will not be called.\nDrag off pins to build functionality.
)

(fn ConstructionScript
  (|CallParentFunction))

(fn Work0
  (|CallParentFunction)
  (Rendering|Material|SetMaterial (Variables|Default|GetCube) 0 "/Game/MainMenu/MenuBallMaterial.MenuBallMaterial"))

(fn Work1
  (|CallParentFunction)
  (Rendering|Material|SetMaterial (Variables|Default|GetCube) 0 "/Game/Geometry/Meshes/CubeMaterial.CubeMaterial"))

(fn Interact
  (bind _issuccesful (|CallParentFunction))
  (if _issuccesful
    (Variables|Default|SetBusy false))
  (return _issuccesful))