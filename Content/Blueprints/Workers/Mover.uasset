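; Mover is a worker Blueprint that slides a MovingPart between two positions, named as opening and closing a bridge.
; BeginPlay derives the timeline play rate from MovingLength and MovingSpeed, then places the part at either end of its local X travel according to OpenedOnStart.
; Work0 and Work1 override parent actions, choosing opposite directions from that flag.
; The timeline lerps the position forward or in reverse and clears Busy when finished, which IsBusy reports.
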(event Custom|open%20bridge
  ;[1 1 1] open/close moving
  (bind _main_track (Timeline|Bridge%20opennig%20timeline PlayFromStart)
    (:Update
      (Transformation|SetRelativeLocation (Variables|Default|GetMoving%20part) (Math|Vector|Lerp(Vector) (Variables|Default|GetStartPosition) (Variables|Default|GetEndPosition) _main_track) false false))
    (:Finished
      (Variables|Default|SetBusy false))))

(event Custom|close%20bridge
  ;[1 1 1] open/close moving
  (bind _main_track (Timeline|Bridge%20opennig%20timeline ReverseFromEnd)
    (:Update
      (Transformation|SetRelativeLocation (Variables|Default|GetMoving%20part) (Math|Vector|Lerp(Vector) (Variables|Default|GetStartPosition) (Variables|Default|GetEndPosition) _main_track) false false))
    (:Finished
      (Variables|Default|SetBusy false))))

(event EventBeginPlay
  (bind _moving_part (Variables|Default|GetMoving%20part))
  (bind _movinglength (Variables|Default|GetMovingLength))
  (|CallParentFunction)
  ;[1 1 1] set up start configuration
  (Components|Timeline|SetPlayRate (Variables|Default|GetBridge%20opennig%20timeline) (/ 1.0 (/ _movinglength (Variables|Default|GetMovingSpeed))))
  (bind _output_get (Variables|Default|SetStartPosition "0, 0, 0"))
  (bind _output_get_2 (Variables|Default|SetEndPosition (Math|Vector|MakeVector _movinglength 0.0 0.0)))
  (if (Variables|Default|GetOpenedOnStart)
    (Transformation|SetRelativeLocation _moving_part _output_get false false)
    (else
      (Transformation|SetRelativeLocation _moving_part _output_get_2 false false))))

(event Collision|EventActorBeginOverlap
  (params (OtherActor :type Actor%20Object%20Reference)))

(event EventTick
  (params (DeltaSeconds :type Float%20%28single-precision%29)))

(fn ConstructionScript
  (|CallParentFunction))

(fn Work0
  (|CallParentFunction)
  (if (Variables|Default|GetOpenedOnStart)
    (CallFunction|OpenBridge)
    (else
      (CallFunction|CloseBridge))))

(fn Work1
  (|CallParentFunction)
  (if (Variables|Default|GetOpenedOnStart)
    (CallFunction|CloseBridge)
    (else
      (CallFunction|OpenBridge))))

(fn IsBusy
  (return (Variables|Default|GetBusy)))