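; Base two-state worker that toggles between two conditions when switched and relays the switch to linked actors.
; An interacting switch calls Interact, which requires parent approval and a non-busy state, then sets Busy, flips Condition and runs the empty Work0 or Work1 hook.
; Successful interactions, and all non-interaction switches, forward a non-interaction Switch to NetChildren through ISwitchable, skipping the Starter.
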(event EventBeginPlay)

(event Collision|EventActorBeginOverlap
  (params (OtherActor :type Actor%20Object%20Reference)))

(event EventTick
  (params (DeltaSeconds :type Float%20%28single-precision%29)))

(event EventSwitch
  (params (Intearction :type Boolean) (Starter :type Actor%20Object%20Reference))
  ;[1 1 1] Start interaction if needed
  (if Intearction
    (bind _issuccesful (CallFunction|Interact))
    (if _issuccesful
      ;[1 1 1] Send switch signal to net children
      (for _array_element (Variables|Default|GetNetChildren) :!label _label
        (bind _asiswitchable (Utilities|Casting|CastToISwitchable _array_element))
        (if (not (== _asiswitchable Starter))
          (Default|Switch _asiswitchable false))))
    (else
      (goto _label))))

(fn ConstructionScript
  (|CallParentFunction))

(fn Work0)

(fn Work1)

(fn Interact
  (bind _issuccesful (|CallParentFunction))
  (if _issuccesful
    (if (Variables|Default|GetBusy)
      (Development|PrintString "error: worker is busy" true true "(R=0.796875,G=0.000000,B=0.000000,A=1.000000)")
      (else
        (Variables|Default|SetBusy true)
        (if (Variables|Default|GetCondition)
          (Variables|Default|SetCondition false)
          (CallFunction|Work1)
          (else
            (Variables|Default|SetCondition true)
            (CallFunction|Work0)))
        (return true))))
  (return false))