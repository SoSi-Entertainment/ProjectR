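; Two-state worker Actor that alternates between two jobs each time it is interacted with.
; Interact refuses with a printed error while IsBusy is set; otherwise it sets the flag, flips Condition, calls Work0 or Work1 and returns true.
; Work0 and Work1 are empty stubs, and nothing in this Blueprint clears IsBusy.
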(event EventBeginPlay)

(event Collision|EventActorBeginOverlap
  (params (OtherActor :type Actor%20Object%20Reference)))

(event EventTick
  (params (DeltaSeconds :type Float%20%28single-precision%29)))

(fn ConstructionScript)

(fn Work0)

(fn Work1)

(fn Interact
  (if (Variables|Default|GetIsBusy)
    (Development|PrintString "error: worker is busy" true true "(R=0.796875,G=0.000000,B=0.000000,A=1.000000)")
    (return false)
    (else
      (Variables|Default|SetIsBusy true)
      (if (Variables|Default|GetCondition)
        (Variables|Default|SetCondition false)
        (CallFunction|Work1)
        (else
          (Variables|Default|SetCondition true)
          (CallFunction|Work0)))
      (return true))))