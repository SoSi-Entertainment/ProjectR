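; EnergyComponent is an energy pool component that stores a current Energy value against a MaxEnergy limit.
; PutEnergy adds an amount and caps the result at MaxEnergy.
; TakeEnerge subtracts an amount only if the result stays at or above zero, returning whether it succeeded.
; GetPercent returns the fill ratio, and the component does no work on BeginPlay or Tick.
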(event EventBeginPlay)

(event EventTick
  (params (DeltaSeconds :type Float%20%28single-precision%29)))

(fn PutEnergy
  (params (value :type Float%20%28double-precision%29))
  (bind _maxenergy (Variables|Default|GetMaxEnergy))
  (Math|Float|CompareFloat (+ value (Variables|Default|GetEnergy)) _maxenergy
    (:>
      (Variables|Default|SetEnergy _maxenergy))
    (:==
      (Variables|Default|SetEnergy (+ value (Variables|Default|GetEnergy)) :!label _label))
    (:<
      (goto _label))))

(fn TakeEnerge
  (params (Value :type Float%20%28double-precision%29))
  (Math|Float|CompareFloat (- (Variables|Default|GetEnergy) Value) 0.0
    (:>
      _)
    (:==
      _)
    (:<
      (return false)))
  (Variables|Default|SetEnergy (- (Variables|Default|GetEnergy) Value))
  (return true))

(fn GetPercent
  (return (/ (Variables|Default|GetEnergy) (Variables|Default|GetMaxEnergy))))