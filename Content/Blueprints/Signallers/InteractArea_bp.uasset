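; Interaction area actor that reports whether the player stands inside its box and shows its text accordingly.
; IsPlayerInCollisionBox tests BoxCollision for overlap with player 0's pawn on demand, as the overlap event is unused.
; The SetVisibility event applies that result to the TextRender's visibility, and Interact returns it to its caller without triggering any other action.
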(event Custom|Set%20Visibility
  ;[1 1 1] Show area text
  (bind _result (CallFunction|IsPlayerinCollisionBox))
  (Rendering|SetVisibility (Variables|Default|GetText%20render) _result false))

(event Collision|EventActorBeginOverlap
  (params (OtherActor :type Actor%20Object%20Reference)))

(fn ConstructionScript
  (|CallParentFunction))

(fn IsPlayerinCollisionBox
  (return (Collision|IsOverlappingActor (Variables|Default|GetBox%20collision) (Game|Player|GetPlayerPawn 0) :!class /Script/Engine.PrimitiveComponent)))

(fn Interact
  (bind _result (CallFunction|IsPlayerinCollisionBox))
  (return _result))