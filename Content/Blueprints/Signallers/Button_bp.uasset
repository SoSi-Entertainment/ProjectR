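; Button is an interactable signaller that passes an interaction on to the actor it is connected to.
; Its Interact override runs the parent check first, then calls Interact on the Connected reference through the Interact_bpi interface.
; It returns true once the call is forwarded, and false if the parent check fails or the target is invalid or lacks the interface, printing an error in the latter two cases.
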(event EventBeginPlay
  (|CallParentFunction))

(event Collision|EventActorBeginOverlap
  (params (OtherActor :type Actor%20Object%20Reference))
  (|CallParentFunction OtherActor) ; This node is disabled and will not be called.\nDrag off pins to build functionality.
)

(event EventTick
  (params (DeltaSeconds :type Float%20%28single-precision%29))
  (|CallParentFunction DeltaSeconds) ; This node is disabled and will not be called.\nDrag off pins to build functionality.
)

(fn ConstructionScript
  (|CallParentFunction))

(fn Interact
  (bind _connected (Variables|Default|Getconnected))
  (bind _issuccesful (|CallParentFunction))
  (if _issuccesful
    (Utilities|IsValid _connected
      (:Is%20Valid
        (bind _asinteract_bpi (Utilities|Casting|CastToInteract_bpi _connected)
          (:then
            (Default|Interact _asinteract_bpi)
            (return true))
          (:CastFailed
            (Development|PrintString "error: parent actor is not worker" true true "(R=0.796875,G=0.000000,B=0.000000,A=1.000000)"))))
      (:Is%20Not%20Valid
        (Development|PrintString "error: no parent actor" true true "(R=0.796875,G=0.000000,B=0.000000,A=1.000000)"))))
  (return false))