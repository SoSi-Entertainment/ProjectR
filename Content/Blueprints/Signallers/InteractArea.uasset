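; InteractArea is a signaller Blueprint that marks a box zone where the player can interact and shows a text prompt there.
; Overlap begin and end events from the player character share one path that sets the TextRender visibility from a box-collision check against player pawn 0.
; Interact returns that same check, reporting whether the player is inside the area.
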(event Collision|EventActorBeginOverlap
  (params (OtherActor :type Actor%20Object%20Reference))
  ;[1 1 1] Show area text
  (Variables|Default|SetOverlapedActor OtherActor)
  (Utilities|Casting|CastToPlayerCharacter (Variables|Default|GetOverlapedActor))
  (bind _result (CallFunction|IsPlayerinCollisionBox))
  (Rendering|SetVisibility (Variables|Default|GetText%20render) _result false))

(event Collision|EventActorEndOverlap
  (params (OtherActor :type Actor%20Object%20Reference))
  ;[1 1 1] Show area text
  (Variables|Default|SetOverlapedActor OtherActor)
  (Utilities|Casting|CastToPlayerCharacter (Variables|Default|GetOverlapedActor))
  (bind _result (CallFunction|IsPlayerinCollisionBox))
  (Rendering|SetVisibility (Variables|Default|GetText%20render) _result false))

(fn ConstructionScript
  (|CallParentFunction))

(fn IsPlayerinCollisionBox
  (return (Collision|IsOverlappingActor (Variables|Default|GetBox%20collision) (Game|Player|GetPlayerPawn 0) :!class /Script/Engine.PrimitiveComponent)))

(fn Interact
  (bind _result (CallFunction|IsPlayerinCollisionBox))
  (return _result))