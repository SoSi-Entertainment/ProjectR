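; Interactable terminal signaller that shows a text prompt in range and passes interaction on to its NetParent.
; Overlap events count actors of DetectionClass in the area, showing the TextRender while any are present.
; Interact calls Switch on a NetParent implementing ISwitchable, otherwise its Interact, and prints an error if none is attached.
; A helper function reports whether the player pawn overlaps the box collision.
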(event Collision|EventActorBeginOverlap
  (params (OtherActor :type Actor%20Object%20Reference))
  (bind _text_render (Variables|Default|GetText%20render))
  (bind _targetsinarea (Variables|Default|GetTargetsInArea))
  ;[1 1 1] Show area text
  (|CallParentFunction OtherActor)
  (if (Utilities|ClassIsChildOf (Utilities|GetClass OtherActor) (Variables|Default|GetDetectionClass))
    (Math|Integer|IncrementInt _targetsinarea
      (:%20%20
        (Math|Integer|CompareInt _targetsinarea
          (:>
            (Rendering|SetVisibility _text_render true false))
          (:==
            (Rendering|SetVisibility _text_render false false)))))))

(event Collision|EventActorEndOverlap
  (params (OtherActor :type Actor%20Object%20Reference))
  (bind _text_render (Variables|Default|GetText%20render))
  (bind _targetsinarea (Variables|Default|GetTargetsInArea))
  ;[1 1 1] Show area text
  (|CallParentFunction OtherActor)
  (if (Utilities|ClassIsChildOf (Utilities|GetClass OtherActor) (Variables|Default|GetDetectionClass))
    (Math|Integer|DecrementInt _targetsinarea
      (:%20%20
        (Math|Integer|CompareInt _targetsinarea
          (:>
            (Rendering|SetVisibility _text_render true false))
          (:==
            (Rendering|SetVisibility _text_render false false)))))))

(fn ConstructionScript
  (|CallParentFunction))

(fn IsPlayerinCollisionBox
  (return (Collision|IsOverlappingActor (Variables|Default|GetBox%20collision) (Game|Player|GetPlayerPawn 0) :!class /Script/Engine.PrimitiveComponent)))

(fn Interact
  (bind _netparent (Variables|Default|GetNetParent))
  (|CallParentFunction)
  (Utilities|IsValid _netparent
    (:Is%20Valid
      (bind _asiswitchable (Utilities|Casting|CastToISwitchable _netparent)
        (:then
          (Default|Switch _asiswitchable true))
        (:CastFailed
          (Default|Interact _netparent)))
      (return true))
    (:Is%20Not%20Valid
      (Development|PrintString "error: not attached" true true "(R=0.796875,G=0.000000,B=0.000000,A=1.000000)")
      (return false))))