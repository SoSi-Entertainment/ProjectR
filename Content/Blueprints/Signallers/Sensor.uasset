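; Sensor is a signaller actor that fires its inherited Interact when actors of a chosen class enter or leave its overlap area.
; Begin and end overlap events check the other actor's class against WhoCanBeDetected, then use TriggeredOn to fire on entry, exit or both.
; Interact only forwards to the parent implementation, and BeginPlay copies WhoCanBeDetected into DetectionClass.
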(event EventBeginPlay
  (|CallParentFunction)
  (Variables|Default|SetDetectionClass (Variables|Default|GetWhoCanBeDetected)))

(event Collision|EventActorBeginOverlap
  (params (OtherActor :type Actor%20Object%20Reference))
  (|CallParentFunction OtherActor)
  (if (Utilities|ClassIsChildOf (Utilities|GetClass OtherActor) (Variables|Default|GetWhoCanBeDetected))
    (switch Utilities|FlowControl|Switch|SwitchonSensorMode (Variables|Default|GetTriggered%20on)
      (:NewEnumerator0
        _)
      (:NewEnumerator1
        _))
    (CallFunction|Interact)))

(event EventTick
  (params (DeltaSeconds :type Float%20%28single-precision%29))
  (|CallParentFunction DeltaSeconds) ; This node is disabled and will not be called.\nDrag off pins to build functionality.
)

(event Collision|EventActorEndOverlap
  (params (OtherActor :type Actor%20Object%20Reference))
  (|CallParentFunction OtherActor)
  (if (Utilities|ClassIsChildOf (Utilities|GetClass OtherActor) (Variables|Default|GetWhoCanBeDetected))
    (switch Utilities|FlowControl|Switch|SwitchonSensorMode (Variables|Default|GetTriggered%20on)
      (:NewEnumerator1
        _)
      (:NewEnumerator2
        _))
    (CallFunction|Interact)))

(fn ConstructionScript
  (|CallParentFunction))

(fn Interact
  (bind _issuccesful (|CallParentFunction))
  (return _issuccesful))