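; Battery is a collectible energy actor whose construction script loads its EnergyComponent with Capacity and calls Set on SetterZeroX.
; Collect transfers all of that energy to the Collector's EnergyComponent and destroys the battery after a short delay.
; Collect also opens a gate on Tick that plays the pickup animation, randomly tumbling the actor while pushing it along its local Z axis.
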(event EventBeginPlay)

(event Collision|EventActorBeginOverlap
  (params (OtherActor :type Actor%20Object%20Reference)))

(event EventTick
  (params (DeltaSeconds :type Float%20%28single-precision%29))
  ;[1 1 1] Collection Animation
  (Utilities|FlowControl|Gate true
    (:Exit
      (Transformation|SetActorRotation (Math|Rotator|CombineRotators (* (* (Math|Random|RandomRotator false) 5.0) DeltaSeconds) (Transformation|GetActorRotation)))
      (Transformation|AddActorLocalOffset (* (Math|Vector|MakeVector 0.0 0.0 1e+03) DeltaSeconds) false false))))

(event EventCollect
  (params (Collector :type Player%20Character%20Bp%20Object%20Reference))
  (Utilities|FlowControl|Sequence
    (:then_0
      (Default|TransitAllEnergy (Variables|Default|GetEnergyComponent) (Variables|/Game/Blueprints/Characters/PlayerCharacter_bp.PlayerCharacter_bp_C|GetEnergyComponent Collector)))
    (:then_1
      ;[1 1 1] Collection Animation
      (Utilities|FlowControl|Gate true) ; enters at Open
    )
    (:then_2
      (Utilities|FlowControl|Delay 1.0)
      (Actor|DestroyActor))))

(fn ConstructionScript
  (Default|Set (Variables|Default|GetSetterZeroX))
  (Default|PutEnergy (Variables|Default|GetEnergyComponent) (Variables|Default|GetCapacity)))