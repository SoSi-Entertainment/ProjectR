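; Energy component that stores an amount capped at a maximum and moves it between energy holders.
; PutEnergy clamps at the cap, while TakeEnergy succeeds only if enough is stored and reports the result.
; Transit functions build on these to send a given amount, everything, or just enough to fill the target, falling back to everything when short.
; Helpers report the space left and the fill ratio.
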(event EventBeginPlay)

(event EventTick
  (params (DeltaSeconds :type Float%20%28single-precision%29)))

(fn PutEnergy
  (params (value :type Float%20%28double-precision%29))
  (bind _maxenergy (Variables|Default|GetMaxEnergy))
  (Math|Float|CompareFloat (+ value (Variables|Default|GetEnergy)) _maxenergy
    (:>
      (Variables|Default|SetEnergy _maxenergy))
    (:==
      (Variables|Default|SetEnergy (+ value (Variables|Default|GetEnergy)) :!label _label))
    (:<
      (goto _label))))

(fn TakeEnergy
  (params (Value :type Float%20%28double-precision%29))
  (Math|Float|CompareFloat (- (Variables|Default|GetEnergy) Value) 0.0
    (:>
      _)
    (:==
      _)
    (:<
      (return false)))
  (Variables|Default|SetEnergy (- (Variables|Default|GetEnergy) Value))
  (return true))

(fn TakeAllEnergy
  (bind _energy (Variables|Default|GetEnergy))
  (bind _output_get (LocalVariables|SetEnergyTaken _energy))
  (CallFunction|TakeEnergy _energy)
  (return _output_get))

(fn TransitEnergy
  (params (Value :type Float%20%28double-precision%29) (To :type Energy%20Component%20Object%20Reference))
  (bind _succes (CallFunction|TakeEnergy Value))
  (if _succes
    (CallFunction|PutEnergy To Value))
  (return _succes))

(fn TransitAllEnergy
  (params (To :type Energy%20Component%20Object%20Reference))
  (bind _value (CallFunction|TakeAllEnergy))
  (CallFunction|PutEnergy To _value))

(fn TransitUntilFull
  (params (To :type Energy%20Component%20Object%20Reference))
  (bind _value (CallFunction|NeedEnergytoFull To))
  (bind _succes (CallFunction|TransitEnergy _value To))
  (if _succes
    _
    (else
      (CallFunction|TransitAllEnergy To)))
  (return _succes))

(fn NeedEnergytoFull
  (return (- (Variables|Default|GetMaxEnergy) (Variables|Default|GetEnergy))))

(fn GetPercent
  (return (/ (Variables|Default|GetEnergy) (Variables|Default|GetMaxEnergy))))